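; BP_ManageableFirst is a manageable object that closes itself after a countdown.
; OnReady enables ticking, and each tick subtracts delta time from WaitTime, prints the remaining value on screen, and calls Close once it reaches zero or below.
; OnOpen always returns true.
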(event `self.OnTick`
  (params (DeltaTime :type "Float (single-precision)"))
  (bind _output_get (set `self.WaitTime` (- (`self.WaitTime`) DeltaTime)))
  (`KismetSystemLibrary.PrintString` null (`KismetStringLibrary.Conv_DoubleToString` _output_get) true false (struct :`G` 0.66 :`B` 1.0 :`A` 1.0) 0.0)
  (if (<= _output_get 0.0)
    (`self.Close`)))

(event `self.OnReady`
  (`self.SetTickable` true))

(fn `OnOpen`
  (returns (ReturnValue :type Boolean))
  (return true))