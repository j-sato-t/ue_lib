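; Actor Blueprint that records its own location to an action log through a directly constructed ActionReplay object.
; On BeginPlay it creates the object in Record mode and opens it with trace-level logging.
; Each Tick saves the actor position as a non-forced vector entry while the logger is valid, and Destroyed closes the log.
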(event `self.ReceiveBeginPlay`
  (bind _returnvalue (`|GenericCreateObject` "/Script/UELib.ActionReplay" "Record" "ActionLog_directObj.log"))
  (bind _output_get (set `self.ActionLogger` _returnvalue))
  (`Manageable.Open` _output_get (make `OpenSetting` "Trace" "ActionLogger")))

(event `self.ReceiveTick`
  (params (DeltaSeconds :type "Float (single-precision)"))
  (bind _actionlogger (`self.ActionLogger`))
  (`/Engine/EditorBlueprintResources/StandardMacros.IsValid` _actionlogger
    (:`Is Valid`
      (`ActionReplay.SaveVector` _actionlogger "ActorPos" (`self.K2_GetActorLocation`) false))))

(event `self.ReceiveDestroyed`
  (`Manageable.Close` (`self.ActionLogger`)))

(fn `UserConstructionScript`)