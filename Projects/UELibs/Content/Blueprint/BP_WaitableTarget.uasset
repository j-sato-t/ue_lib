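; BP_WaitableTarget is a waitable task Blueprint that completes after about one second, apparently as a test or example.
; StartTask enables ticking, and OnTick accumulates delta time into WaitTime, printing a wait message while it runs.
; Once the threshold is passed, it prints an end message, disables ticking and calls SetFinish to signal completion.
; WaitTime is never reset within this graph.
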(event `self.StartTask`
  (`self.SetTickable` true))

(event `self.OnTick`
  (params (DeltaTime :type "Float (single-precision)"))
  (bind _output_get (set `self.WaitTime` (+ DeltaTime (`self.WaitTime`))))
  (if (> _output_get 1.0)
    (`KismetSystemLibrary.PrintString` null "end task")
    (`self.SetTickable` false)
    (`self.SetFinish`)
    (else
      (`KismetSystemLibrary.PrintString` null "wait task" true true (struct :`G` 0.66 :`B` 1.0 :`A` 1.0) 0.0))))